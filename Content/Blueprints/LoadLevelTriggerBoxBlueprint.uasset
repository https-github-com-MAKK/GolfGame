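; Trigger box Blueprint that starts a level load when a designated actor overlaps it, with an option to roll credits first.
; On overlap it compares the actor to ActorToCheck, then branches on RollCredits.
; The credits path waits before adding a widget to the viewport, while the normal path shows a loading screen widget immediately.
; Both paths then wait a configurable delay before calling LevelLoad.
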(event `self.ReceiveActorBeginOverlap`
  (params (OtherActor :type "Actor Object Reference"))
  (if (== OtherActor (`self.ActorToCheck`))
    (bind _output_get (set `self.IsCharacterInTrigger` true))
    (if (and _output_get (`self.RollCredits`))
      (`KismetSystemLibrary.Delay` (`self.EndCreditsDelay`))
      (bind _returnvalue (`|CreateWidget` "/Game/Level_Transition/EndCredits/Credits.Credits_C"))
      (`UserWidget.AddToViewport` _returnvalue 0)
      (`KismetSystemLibrary.Delay` (`self.LevelLoadTimeDelay`))
      (`self.LevelLoad`)
      (elif (`self.IsCharacterInTrigger`)
        (bind _returnvalue_2 (`|CreateWidget` "/Game/Level_Transition/LoadingScreen/LoadingScreenWidget.LoadingScreenWidget_C"))
        (`UserWidget.AddToViewport` _returnvalue_2 0)
        (`KismetSystemLibrary.Delay` (`self.LevelLoadTimeDelay`))
        (`self.LevelLoad`)))))

(fn `UserConstructionScript`)