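; ActivateDoor is an overlap trigger that lets a Door open and powers a set of lights while a Ball is inside it.
; Begin and end overlap events cast to Ball, then toggle the Door's CanOpen flag and switch the referenced spot and point lights on or off through their intensity.
; Both events set the WindTriggerBox's IsUsable to false, so leaving the trigger does not re-enable it.
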(event `self.ReceiveActorEndOverlap`
  (params (OtherActor :type "Actor Object Reference"))
  (cast `Ball` OtherActor)
  (set `/Game/ProxmityTriggeredDoor.CanOpen` false (`self.door`))
  (set `WindTriggerBox.IsUsable` false (`self.windTriggerBox`))
  (`LightComponent.SetIntensity` (`SpotLight.SpotLightComponent` (`self.spotLight1`)) 0.0)
  (`LightComponent.SetIntensity` (`SpotLight.SpotLightComponent` (`self.spotLight2`)) 0.0)
  (`LightComponent.SetIntensity` (`PointLight.PointLightComponent` (`self.pointLight1`)) 0.0)
  (`LightComponent.SetIntensity` (`PointLight.PointLightComponent` (`self.pointLight2`)) 0.0)
  (`LightComponent.SetIntensity` (`PointLight.PointLightComponent` (`self.pointLight3`)) 0.0)
  (`LightComponent.SetIntensity` (`PointLight.PointLightComponent` (`self.pointLight4`)) 0.0)
  (`LightComponent.SetIntensity` (`PointLight.PointLightComponent` (`self.pointLight5`)) 0.0)
  (`LightComponent.SetIntensity` (`PointLight.PointLightComponent` (`self.pointLight6`)) 0.0)
  (`LightComponent.SetIntensity` (`PointLight.PointLightComponent` (`self.pointLight7`)) 0.0)
  (`LightComponent.SetIntensity` (`PointLight.PointLightComponent` (`self.pointLight8`)) 0.0)
  (`LightComponent.SetIntensity` (`PointLight.PointLightComponent` (`self.pointLight9`)) 0.0)
  (`LightComponent.SetIntensity` (`Light.LightComponent` (`self.pointLight10`)) 0.0)
  (`LightComponent.SetIntensity` (`Light.LightComponent` (`self.pointLight11`)) 0.0))

(event `self.ReceiveActorBeginOverlap`
  (params (OtherActor :type "Actor Object Reference"))
  (cast `Ball` OtherActor)
  (set `/Game/ProxmityTriggeredDoor.CanOpen` true (`self.door`))
  (set `WindTriggerBox.IsUsable` false (`self.windTriggerBox`))
  (`LightComponent.SetIntensity` (`SpotLight.SpotLightComponent` (`self.spotLight1`)) 200.0)
  (`LightComponent.SetIntensity` (`SpotLight.SpotLightComponent` (`self.spotLight2`)) 200.0)
  (`LightComponent.SetIntensity` (`PointLight.PointLightComponent` (`self.pointLight1`)) 200.0)
  (`LightComponent.SetIntensity` (`PointLight.PointLightComponent` (`self.pointLight2`)) 200.0)
  (`LightComponent.SetIntensity` (`PointLight.PointLightComponent` (`self.pointLight3`)) 200.0)
  (`LightComponent.SetIntensity` (`PointLight.PointLightComponent` (`self.pointLight4`)) 200.0)
  (`LightComponent.SetIntensity` (`PointLight.PointLightComponent` (`self.pointLight5`)) 200.0)
  (`LightComponent.SetIntensity` (`PointLight.PointLightComponent` (`self.pointLight6`)) 200.0)
  (`LightComponent.SetIntensity` (`PointLight.PointLightComponent` (`self.pointLight7`)) 200.0)
  (`LightComponent.SetIntensity` (`PointLight.PointLightComponent` (`self.pointLight8`)) 200.0)
  (`LightComponent.SetIntensity` (`PointLight.PointLightComponent` (`self.pointLight9`)) 200.0)
  (`LightComponent.SetIntensity` (`Light.LightComponent` (`self.pointLight10`)) 200.0)
  (`LightComponent.SetIntensity` (`Light.LightComponent` (`self.pointLight11`)) 200.0))

(fn `UserConstructionScript`)