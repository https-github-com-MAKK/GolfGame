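; Door to the next level that opens while the ball-in-goal flag is set and the actor overlaps its target actor.
; Tick polls both conditions, activating two steam door components and playing a timeline when they hold, and reversing the timeline otherwise.
; The timeline lerps the small door mesh's relative location between closed and open positions.
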(event `self.ReceiveTick`
  (params (DeltaSeconds :type "Float (single-precision)"))
  (if (and (`self.IsBallInGoalTrigger`) (`self.IsOverlappingActor` (`self.TargetActor`)))
    (`ActorComponent.Activate` (`self.SteamDoor`) false)
    (`ActorComponent.Activate` (`self.SteamDoor2`) false)
    (bind (_direction _doorposition) (`Timeline|Timeline_0` :!label _label)
      (:`Update`
        (`SceneComponent.K2_SetRelativeLocation` (`self.Door_Small_A`) (`KismetMathLibrary.VLerp` (`self.DoorClosed`) (`self.DoorOpen`) _doorposition) false false)))
    (else
      (goto _label :!via `Reverse`))))

(fn `UserConstructionScript`)